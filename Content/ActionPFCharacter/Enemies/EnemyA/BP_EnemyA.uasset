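; BP_EnemyA is an enemy Blueprint with an overhead HP bar widget.
; On BeginPlay it casts the widget to Widget_HPBar_Basic and registers itself with it as the tracked character.
; Each Tick it sets the widget's world yaw to the first player controller's yaw plus 180 degrees, with zero pitch and roll, billboarding the bar toward the player's view.
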(event EventBeginPlay
  (bind _aswidget_hpbar_basic (Utilities|Casting|CastToWidget_HPBar_Basic (UserInterface|GetWidget (Variables|Default|GetHPBarWidget))))
  (Class|WidgetHPBarBasic|RegistCharacter _aswidget_hpbar_basic self))

(event Collision|EventActorBeginOverlap
  (params (OtherActor :type Actor%20Object%20Reference)))

(event EventTick
  (params (DeltaSeconds :type Float%20%28single-precision%29))
  (Transformation|SetWorldRotation (Variables|Default|GetHPBarWidget) (Math|Rotator|MakeRotator 0.0 0.0 (+ (.Yaw (Math|Rotator|BreakRotator (Transformation|GetActorRotation (Game|GetPlayerController 0)))) 1.8e+02)) false false))

(fn ConstructionScript)